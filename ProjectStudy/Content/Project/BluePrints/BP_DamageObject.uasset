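; Hazard actor that repeatedly damages an actor overlapping its Box component.
; Begin overlap starts the Damaging timeline, whose updates apply fixed damage through a DoOnce that resets after a short delay to throttle the ticks.
; Any end overlap stops the timeline.
; Disappear and Appear functions toggle the actor's visibility, collision and tick together.
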(event OnComponentBeginOverlap(Box)
  (params (OverlappedComponent :type Primitive%20Component%20Object%20Reference) (OtherActor :type Actor%20Object%20Reference) (OtherComp :type Primitive%20Component%20Object%20Reference) (OtherBodyIndex :type Integer) (bFromSweep :type Boolean) (SweepResult :type Hit%20Result%20Structure%20%28by%20ref%29))
  (Timeline|Damaging PlayFromStart
    (:Update
      (Utilities|FlowControl|DoOnce false :!label _label
        (:Completed
          (Game|Damage|ApplyDamage OtherActor 5.0 0 0)
          (Utilities|FlowControl|Delay 0.1)
          (goto _label Reset))))))

(event OnComponentEndOverlap(Box)
  (params (OverlappedComponent :type Primitive%20Component%20Object%20Reference) (OtherActor :type Actor%20Object%20Reference) (OtherComp :type Primitive%20Component%20Object%20Reference) (OtherBodyIndex :type Integer))
  (Timeline|Damaging Stop
    (:Update
      (Utilities|FlowControl|DoOnce false :!label _label
        (:Completed
          (Game|Damage|ApplyDamage (stale OnComponentBeginOverlap(Box) OtherActor) 5.0 0 0)
          (Utilities|FlowControl|Delay 0.1)
          (goto _label Reset))))))

(fn ConstructionScript)

(fn Disappear
  (Rendering|SetActorHiddenInGame true)
  (Collision|SetActorEnableCollision false)
  (Actor|Tick|SetActorTickEnabled false))

(fn Appear
  (Rendering|SetActorHiddenInGame false)
  (Collision|SetActorEnableCollision true)
  (Actor|Tick|SetActorTickEnabled true))